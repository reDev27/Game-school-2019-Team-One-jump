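; Cannocchialei enemy character that roams to random points and fires a beam at the player.
; A looping timer starts each move; on arrival it faces the player and drives its anim Blueprint through shot and dazed (IsIntontito) states.
; The Cascade beam runs from its Sphere to a one-time snapshot of the player's position, where the Box also moves.
; The Box overlap handler is unfinished and has no effect.
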(event OnComponentBeginOverlap(Box)
  (params (OverlappedComponent :type Primitive%20Component%20Object%20Reference) (OtherActor :type Actor%20Object%20Reference) (OtherComp :type Primitive%20Component%20Object%20Reference) (OtherBodyIndex :type Integer) (bFromSweep :type Boolean) (SweepResult :type Hit%20Result%20Structure%20%28by%20ref%29))
  (Utilities|Casting|CastToprot_mio_finito OtherActor)
  (bind _asprot_mio_abp (Utilities|Casting|CastToprot_mio_ABP (Components|SkeletalMesh|GetAnimInstance (Variables|/Script/Engine.Character|GetMesh (Game|GetPlayerCharacter 0)))))
  (if (and false (Variables|/Game/prot_mio/animation/prot_mio_ABP.prot_mio_ABP_C|Getis_punching _asprot_mio_abp))
    _))

(event Custom|movement
  (bind _returnvalue (Game|GetPlayerCharacter 0))
  (bind _returnvalue_2 (Transformation|GetActorLocation _returnvalue))
  (AI|AIMoveTo (AI|GetAIController self) (Math|Vector|MakeVector (Math|Random|RandomFloatinRange -1.8e+03 1.8e+03) (Math|Random|RandomFloatinRange -1.8e+03 1.8e+03) 0.0) 0 1.0 "Default" "Default" true true
    (:OnMoveFinished
      (Transformation|SetRelativeRotation (Variables|Collision|GetCapsuleComponent) (Math|Rotator|FindLookatRotation (Transformation|GetActorLocation) (Transformation|GetActorLocation (Game|GetPlayerCharacter 0))) false false)
      (Variables|Default|Setrot (.rotation (Transformation|GetRelativeTransform (Variables|Collision|GetCapsuleComponent))))
      (bind _ascannocchialei_abp (Utilities|Casting|CastTocannocchialei_ABP (Components|SkeletalMesh|GetAnimInstance (Variables|Character|GetMesh))))
      (Variables|Default|Setabp_ref _ascannocchialei_abp)
      (Variables|/Game/characters/cannocchialei/animation/cannocchialei_ABP.cannocchialei_ABP_C|Setshot_beam? _ascannocchialei_abp true)
      (Utilities|FlowControl|Delay 1.0)
      (bind _returnvalue_3 (Effects|SpawnEmitteratLocation "/Game/characters/cannocchialei/emitter/cannocchilei_beam.cannocchilei_beam" "0, 0, 0"))
      (Class|ParticleSystemComponent|SetBeamSourcePoint _returnvalue_3 0 (Transformation|GetWorldLocation (Variables|Default|GetSphere)))
      (Class|ParticleSystemComponent|SetBeamTargetPoint _returnvalue_3 0 _returnvalue_2)
      (Transformation|SetWorldLocation (Variables|Default|GetBox) _returnvalue_2 false false)
      (Utilities|FlowControl|Delay 4.0)
      (Variables|/Game/characters/cannocchialei/animation/cannocchialei_ABP.cannocchialei_ABP_C|Setshot_beam? _ascannocchialei_abp false)
      (Components|DestroyComponent _returnvalue_3)
      (Transformation|SetRelativeRotation (Variables|Collision|GetCapsuleComponent) (Math|Rotator|MakeRotator 0.0 0.0 (.yaw (Variables|Default|Getrot))) false false)
      (Components|Movement|StopMovementImmediately (Variables|Character|GetCharacterMovement))
      (Variables|/Game/characters/cannocchialei/animation/cannocchialei_ABP.cannocchialei_ABP_C|Setis_intontito? (Variables|Default|Getabp_ref) true)
      (Utilities|FlowControl|Delay 3.9)
      (Variables|/Game/characters/cannocchialei/animation/cannocchialei_ABP.cannocchialei_ABP_C|Setis_intontito? (Variables|Default|Getabp_ref) false))))

(event EventBeginPlay
  (Utilities|Time|SetTimerbyFunctionName 0 "movement" 9.0 true))

(fn ConstructionScript)