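; Electric hazard actor that periodically fires a beam at the player's position and damages them.
; A looping timer snapshots the player location, picks one of four sphere emitters, then after a dodgeable delay draws a particle beam to that spot.
; A Box hitbox jumps to the target and subtracts health from prot_mio_finito's selected life pool on overlap, then shifts upward as the beam is destroyed.
; The SpawnerBeam helper is not called here.
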(event OnComponentBeginOverlap(Box)
  (params (OverlappedComponent :type Primitive%20Component%20Object%20Reference) (OtherActor :type Actor%20Object%20Reference) (OtherComp :type Primitive%20Component%20Object%20Reference) (OtherBodyIndex :type Integer) (bFromSweep :type Boolean) (SweepResult :type Hit%20Result%20Structure%20%28by%20ref%29))
  (bind _asprot_mio_finito (Utilities|Casting|CastToprot_mio_finito OtherActor))
  (switch int (Variables|/Game/prot_mio/prot_mio_finito.prot_mio_finito_C|Getselezione_vita _asprot_mio_finito)
    (:0
      (Variables|/Game/prot_mio/prot_mio_finito.prot_mio_finito_C|Setvita_1 _asprot_mio_finito (- (Variables|/Game/prot_mio/prot_mio_finito.prot_mio_finito_C|Getvita_1 _asprot_mio_finito) 25.0)))
    (:1
      (Variables|/Game/prot_mio/prot_mio_finito.prot_mio_finito_C|Setvita_2 _asprot_mio_finito (- (Variables|/Game/prot_mio/prot_mio_finito.prot_mio_finito_C|Getvita_2 _asprot_mio_finito) 25.0)))
    (:2
      (Variables|/Game/prot_mio/prot_mio_finito.prot_mio_finito_C|Setvita_3 _asprot_mio_finito (- (Variables|/Game/prot_mio/prot_mio_finito.prot_mio_finito_C|Getvita_3 _asprot_mio_finito) 25.0)))))

(event Custom|spawn_electric_beam
  ;[1 0.2104 0.7378] spawner del raggio elettrico
  (Variables|Default|Setcharacter_loc (Transformation|GetActorLocation (Game|GetPlayerCharacter 0)))
  (switch int (Math|Random|RandomIntegerinRange 0 3)
    (:0
      (bind _output_get (Variables|Default|Setsource_location (Transformation|GetWorldLocation (Variables|Default|GetSphere))))
      (Utilities|FlowControl|Delay 1.0)
      (bind _returnvalue (Effects|SpawnEmitteratLocation "/Game/characters/teslaman/teslona/emitter/electric_emitter.electric_emitter" _output_get))
      (Class|ParticleSystemComponent|SetBeamSourcePoint _returnvalue 0 _output_get)
      (Class|ParticleSystemComponent|SetBeamTargetPoint _returnvalue 0 (Variables|Default|Getcharacter_loc))
      (Transformation|SetWorldLocation (Variables|Default|GetBox) (Variables|Default|Getcharacter_loc) false false)
      (Utilities|FlowControl|Delay 2.9)
      (Transformation|SetWorldLocation (Variables|Default|GetBox) (+ (Variables|Default|Getcharacter_loc) "0, 0,100.000000") false false)
      (Components|DestroyComponent _returnvalue))
    (:1
      (bind _output_get_2 (Variables|Default|Setsource_location (Transformation|GetWorldLocation (Variables|Default|GetSphere1))))
      (Utilities|FlowControl|Delay 1.0)
      (bind _returnvalue_2 (Effects|SpawnEmitteratLocation "/Game/characters/teslaman/teslona/emitter/electric_emitter.electric_emitter" _output_get_2))
      (Class|ParticleSystemComponent|SetBeamSourcePoint _returnvalue_2 0 _output_get_2)
      (Class|ParticleSystemComponent|SetBeamTargetPoint _returnvalue_2 0 (Variables|Default|Getcharacter_loc))
      (Transformation|SetWorldLocation (Variables|Default|GetBox) (Variables|Default|Getcharacter_loc) false false)
      (Utilities|FlowControl|Delay 2.9)
      (Transformation|SetWorldLocation (Variables|Default|GetBox) (+ (Variables|Default|Getcharacter_loc) "0, 0,100.000000") false false)
      (Components|DestroyComponent _returnvalue_2))
    (:2
      (bind _output_get_3 (Variables|Default|Setsource_location (Transformation|GetWorldLocation (Variables|Default|GetSphere2))))
      (Utilities|FlowControl|Delay 1.0)
      (bind _returnvalue_3 (Effects|SpawnEmitteratLocation "/Game/characters/teslaman/teslona/emitter/electric_emitter.electric_emitter" _output_get_3))
      (Class|ParticleSystemComponent|SetBeamSourcePoint _returnvalue_3 0 _output_get_3)
      (Class|ParticleSystemComponent|SetBeamTargetPoint _returnvalue_3 0 (Variables|Default|Getcharacter_loc))
      (Transformation|SetWorldLocation (Variables|Default|GetBox) (Variables|Default|Getcharacter_loc) false false)
      (Utilities|FlowControl|Delay 2.9)
      (Transformation|SetWorldLocation (Variables|Default|GetBox) (+ (Variables|Default|Getcharacter_loc) "0, 0,100.000000") false false)
      (Components|DestroyComponent _returnvalue_3))
    (:3
      (bind _output_get_4 (Variables|Default|Setsource_location (Transformation|GetWorldLocation (Variables|Default|GetSphere3))))
      (Utilities|FlowControl|Delay 1.0)
      (bind _returnvalue_4 (Effects|SpawnEmitteratLocation "/Game/characters/teslaman/teslona/emitter/electric_emitter.electric_emitter" _output_get_4))
      (Class|ParticleSystemComponent|SetBeamSourcePoint _returnvalue_4 0 _output_get_4)
      (Class|ParticleSystemComponent|SetBeamTargetPoint _returnvalue_4 0 (Variables|Default|Getcharacter_loc))
      (Transformation|SetWorldLocation (Variables|Default|GetBox) (Variables|Default|Getcharacter_loc) false false)
      (Utilities|FlowControl|Delay 2.9)
      (Transformation|SetWorldLocation (Variables|Default|GetBox) (+ (Variables|Default|Getcharacter_loc) "0, 0,100.000000") false false)
      (Components|DestroyComponent _returnvalue_4))))

(event EventBeginPlay
  ;[1 0.1582 0.0565] imposta il timer inizia
  (Utilities|Time|SetTimerbyFunctionName 0 "spawn_electric_beam" 4.0 true))

(fn ConstructionScript)

(fn SpawnerBeam
  (params (Location :type Vector))
  (bind _returnvalue (Game|GetPlayerCharacter 0))
  (bind _returnvalue_2 (Transformation|GetActorLocation _returnvalue))
  (bind _returnvalue_3 (Effects|SpawnEmitteratLocation "/Game/characters/teslaman/teslona/emitter/electric_emitter.electric_emitter" Location))
  (Class|ParticleSystemComponent|SetBeamSourcePoint _returnvalue_3 0 Location)
  (Class|ParticleSystemComponent|SetBeamTargetPoint _returnvalue_3 0 _returnvalue_2)
  (Class|ParticleSystemComponent|SetBeamTargetTangent _returnvalue_3 0 _returnvalue_2)
  (Class|ParticleSystemComponent|SetBeamSourceTangent _returnvalue_3 0 Location)
  (return _returnvalue_3))