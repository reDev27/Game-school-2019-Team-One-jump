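; Melaton boss enemy that periodically chases the player and returns to the HUB level when defeated.
; A looping timer runs a chase, then a rolling charge, then a confused, vulnerable window, driving uomo_mela_ABP animation flags; both random branches lead to the same charge.
; Collision overlaps reduce Vita only while it is vulnerable and the player's prot_mio_ABP reports punching.
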(event OnComponentBeginOverlap(enemy_collision)
  (params (OverlappedComponent :type Primitive%20Component%20Object%20Reference) (OtherActor :type Actor%20Object%20Reference) (OtherComp :type Primitive%20Component%20Object%20Reference) (OtherBodyIndex :type Integer) (bFromSweep :type Boolean) (SweepResult :type Hit%20Result%20Structure%20%28by%20ref%29))
  (bind _asprot_mio_finito (Utilities|Casting|CastToprot_mio_finito OtherActor))
  (bind _asprot_mio_abp (Utilities|Casting|CastToprot_mio_ABP (Components|SkeletalMesh|GetAnimInstance (Variables|/Script/Engine.Character|GetMesh _asprot_mio_finito))))
  (if (and (Variables|Default|Getis_damangeble) (Variables|/Game/prot_mio/animation/prot_mio_ABP.prot_mio_ABP_C|Getis_punching _asprot_mio_abp))
    (bind _output_get (Variables|Default|Setvita (- (Variables|Default|Getvita) 1e+01)))
    (Development|PrintString (Utilities|String|ToString(Float) (Variables|Default|Getvita)))
    (if (<= _output_get 0.0)
      (Actor|DestroyActor)
      (Game|OpenLevel(byName) "HUB"))))

(event Custom|move_to
  ;[1 1 1] AI
  (AI|Navigation|MovetoActor (AI|GetAIController self) (Game|GetPlayerCharacter 0) 5.0 true true true 0)
  (Utilities|FlowControl|Delay 5.0)
  (AI|Navigation|StopMovement (AI|GetAIController self))
  (bind _asuomo_mela_abp (Utilities|Casting|CastTouomo_mela_ABP (Components|SkeletalMesh|GetAnimInstance (Variables|Character|GetMesh))))
  (switch int (Math|Random|RandomIntegerinRange 0 1)
    (:0
      _)
    (:1
      _))
  (AI|AIMoveTo (AI|GetAIController self) "0, 0, 0" (Game|GetPlayerCharacter 0) 5.0 "Default" "Default" true true
    (:then
      (Variables|/Game/characters/melaton_C/animation/uomo_mela_ABP.uomo_mela_ABP_C|Setis_rotalamento? _asuomo_mela_abp true)
      (Utilities|FlowControl|Delay 5.0)
      (AI|Navigation|StopMovement (AI|GetAIController self))
      (Variables|/Game/characters/melaton_C/animation/uomo_mela_ABP.uomo_mela_ABP_C|Setis_rotalamento? _asuomo_mela_abp false)
      (Variables|/Game/characters/melaton_C/animation/uomo_mela_ABP.uomo_mela_ABP_C|Setis_confused _asuomo_mela_abp true)
      (Variables|Default|Setis_damangeble true)
      (Utilities|FlowControl|Delay 3.9)
      (Variables|/Game/characters/melaton_C/animation/uomo_mela_ABP.uomo_mela_ABP_C|Setis_confused _asuomo_mela_abp false)
      (Variables|Default|Setis_damangeble false))))

(event EventBeginPlay
  ;[1 1 1] AI
  (Utilities|Time|SetTimerbyFunctionName 0 "move_to" 14.0 true))

(fn ConstructionScript)