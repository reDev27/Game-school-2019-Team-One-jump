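; Destructible generator for the electricity room that plays an attached hum and starts the first Tesla music track on BeginPlay.
; A box hit from the player character destroys it if the player's AnimBP reports punching.
; It then increments a Counter meant to step through successive music tracks.
; Counter is per-instance and increments before the switch, so only case 1 is reached, starting track 3 without stopping track 1.
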(event OnComponentHit(Box)
  (params (HitComponent :type Primitive%20Component%20Object%20Reference) (OtherActor :type Actor%20Object%20Reference) (OtherComp :type Primitive%20Component%20Object%20Reference) (NormalImpulse :type Vector :default "0, 0, 0") (Hit :type Hit%20Result%20Structure%20%28by%20ref%29))
  (Utilities|Casting|CastToprot_mio_finito OtherActor)
  (bind _asprot_mio_abp (Utilities|Casting|CastToprot_mio_ABP (Components|SkeletalMesh|GetAnimInstance (Variables|/Script/Engine.Character|GetMesh (Game|GetPlayerCharacter 0)))))
  (if (Variables|/Game/prot_mio/animation/prot_mio_ABP.prot_mio_ABP_C|Getis_punching _asprot_mio_abp)
    (Actor|DestroyActor)
    (Math|Integer|IncrementInt (Variables|Default|Getcounter)
      (:%20%20
        (switch int (Variables|Default|Getcounter)
          (:0
            (Components|DestroyComponent (stale EventBeginPlay _returnvalue))
            (bind _returnvalue (Audio|SpawnSoundatLocation "/Game/mesh_levels/stanza_elettricità/sounds/tesla_musica_2_Cue.tesla_musica_2_Cue" "0, 0,1.000000" "0, 0, 0" 1.0 1.0 0.0 0 0)))
          (:1
            (Components|DestroyComponent _returnvalue)
            (bind _returnvalue_2 (Audio|SpawnSoundatLocation "/Game/mesh_levels/stanza_elettricità/sounds/tesla_musica_3_Cue.tesla_musica_3_Cue" "0.000000, 0,2.000000" "0, 0, 0" 1.0 1.0 0.0 0 0)))
          (:2
            (Components|DestroyComponent _returnvalue_2)
            (Audio|SpawnSoundatLocation "/Game/mesh_levels/stanza_elettricità/sounds/tesla_musica_4_Cue.tesla_musica_4_Cue" "0, 0,3.000000" "0, 0, 0" 1.0 1.0 0.0 0 0)))))))

(event EventBeginPlay
  (Audio|SpawnSoundAttached "/Game/mesh_levels/stanza_elettricità/sounds/suono_generatore_Cue.suono_generatore_Cue" (Variables|Default|GetBox) "None" "0, 0, 0" "0, 0, 0" "KeepRelativeOffset" false 1.0 1.0 0.0 "/Game/mesh_levels/torre_pisa/sounds/sound_class/attenuation_generatori.attenuation_generatori" 0)
  (bind _returnvalue (Audio|SpawnSoundatLocation "/Game/mesh_levels/stanza_elettricità/sounds/tesla_musica_1_Cue.tesla_musica_1_Cue" "0, 0, 0" "0, 0, 0" 1.0 1.0 0.0 0 0 false)))

(fn ConstructionScript)